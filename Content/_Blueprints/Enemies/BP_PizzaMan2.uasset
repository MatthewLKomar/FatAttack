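; BP_PizzaMan2 is an enemy Blueprint variant that takes nearly all of its behavior from its parent class.
; Its overrides for startup, setup, death, ranged throw and melee only call the parent versions.
; OnHurt also calls the parent but passes zero instead of the received DamageAmount.
; Setup holds unconnected, never-executed logic that would spawn an equipped BP_Weapon and attach it to the mesh's GripPoint socket.
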(event EventBeginPlay
  (|CallParentFunction))

(fn ConstructionScript
  (|CallParentFunction))

(fn OnKilled
  (|CallParentFunction))

(fn Setup
  (|CallParentFunction))

(fn ThrowRangedItem
  (|CallParentFunction))

(fn OnHurt
  (params (DamageAmount :type Integer))
  (|CallParentFunction 0))

(fn MeleeAttack
  (|CallParentFunction))