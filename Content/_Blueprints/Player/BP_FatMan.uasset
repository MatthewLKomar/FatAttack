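; First-person player character Blueprint that loads saved player data on BeginPlay and re-equips the current weapon.
; An array of weapon info backs pickup and switching, which destroy the held BP_Weapon and spawn another attached to the hands.
; Interact sphere-traces from the camera for weapons or BPI_Stats objects.
; Firing drives animation flags and calls Shoot even for melee, while damage reduces health and calls overridable hurt and death hooks.
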(event Custom|OnLoad
  (bind _asbp_game_instance (Utilities|Casting|CastToBP_GameInstance (Game|GetGameInstance)))
  (bind _output_get (Variables|Default|SetGame%20Instance _asbp_game_instance))
  (bind _success (Default|LoadPlayerData _output_get))
  (if _success
    (bind _gunref (Weapon|EquipWeaponfromInventory (Variables|Default|GetCurrWeapon)))
    (Utilities|IsValid _gunref
      (:Is%20Valid
        (Variables|Default|SetHeldGun _gunref)))))

(event EventBeginPlay
  (|CallParentFunction)
  ;[1 1 1] Load
  (CallFunction|OnLoad))

(event EventDamage
  (params (Damage :type Integer))
  (_DEBUG|DamagePlayer Damage))

(event Input|ActionEvents|InputActionMightyBoot
  (params (Key :type Key%20Structure :default "None"))
  (:Pressed
    (Default|ClearSaveData (Variables|Default|GetGame%20Instance))))

(event Input|ActionEvents|InputActionFire
  (params (Key :type Key%20Structure :default "None"))
  (bind _heldgun (Variables|Default|GetHeldGun))
  (:Pressed
    (if (Variables|Default|GetIsHoldingGun)
      ;[1 1 1] These need to be done in the anim BP
      (Variables|Default|SetIsShootingGun true)
      (Default|Shoot _heldgun)
      (Utilities|FlowControl|Delay 1.0) ; or however long the animation is
      (Variables|Default|SetIsShootingGun false)
      (else
        (Variables|Default|SetIsHittingMelee true)
        (Utilities|FlowControl|Delay 1.0)
        (Default|Shoot _heldgun) ; MLK; our weapons aren't collisions based. TOO BAD
        (Variables|Default|SetIsHittingMelee false)))))

(event Input|ActionEvents|InputActionPickup
  (params (Key :type Key%20Structure :default "None"))
  (:Pressed
    (CallFunction|Interact)))

(event Input|ActionEvents|InputActionWeapon1
  (params (Key :type Key%20Structure :default "None"))
  (:Pressed
    (Weapon|SwitchWeapon)))

(event Input|ActionEvents|InputActionWeapon2
  (params (Key :type Key%20Structure :default "None"))
  (:Pressed
    (Weapon|SwitchWeapon 1)))

(event Input|ActionEvents|InputActionWeapon3
  (params (Key :type Key%20Structure :default "None"))
  (:Pressed
    (Weapon|SwitchWeapon 2)))

(event Input|ActionEvents|InputActionNextWeapon
  (params (Key :type Key%20Structure :default "None"))
  (:Pressed
    (Weapon|SwitchWeapon (+ (Variables|Default|GetCurrWeapon) 1))
    (_DEBUG|PrintCurrWeapon)))

(event Input|ActionEvents|InputActionPrevWeapon
  (params (Key :type Key%20Structure :default "None"))
  (:Pressed
    (Weapon|SwitchWeapon (- (Variables|Default|GetCurrWeapon) 1))
    (_DEBUG|PrintCurrWeapon)))

(fn ConstructionScript
  (|CallParentFunction))

(fn EquipWeaponfromInventory
  (params (WhichWeapon :type Integer))
  ;[1 1 1] So we don't go out of bounds
  (if (!= (Utilities|Array|Length (Variables|Default|GetWeapons)) 0)
    (bind _output_get (Variables|Default|SetWeaponSelected (Utilities|Array|Get(acopy) (Variables|Default|GetWeapons) (Math|Integer|%(Integer) WhichWeapon (+ (Variables|Default|GetMaxWeapons) 1)))))
    (bind _gunref (Weapon|SpawnWeapon _output_get))
    (return _gunref)
    (else
      (return 0))))

(fn SpawnWeapon
  (params (Weapon :type Weapon%20Definition%20Structure))
  (bind (_id _name _damage _isranged) (Utilities|Struct|BreakWeaponDefinition Weapon))
  (if _isranged
    (Variables|Default|SetIsHoldingGun true)
    (else
      (Variables|Default|SetIsHoldingMelee true)))
  (bind _returnvalue (Game|SpawnActorfromClass "/Game/_Blueprints/Guns/BP_Weapon.BP_Weapon_C" (Math|Transform|MakeTransform "0, 0, 0") "AlwaysSpawn" 0 (Variables|Default|GetHeadTransform) _id true self))
  (Transformation|AttachComponentToComponent _returnvalue (Variables|Default|GetHands) "GripPoint" "KeepRelative" "KeepRelative" "KeepRelative" true)
  (return _returnvalue))

(fn SetWeapon
  (params (WeaponSelected :type Weapon%20Definition%20Structure) (Index :type Integer))
  (bind _output_get (Variables|Default|SetWeaponSelected WeaponSelected))
  (Utilities|Array|SetArrayElem (Variables|Default|GetWeapons) Index _output_get true))

(fn DeselectWeapon
  (bind _heldgun (Variables|Default|GetHeldGun))
  (Utilities|IsValid _heldgun
    (:Is%20Valid
      (if (.isRanged (Utilities|Struct|BreakWeaponDefinition (Variables|Default|GetWeaponSelected)))
        (Variables|Default|SetIsHoldingGun false)
        (else
          (Variables|Default|SetIsHoldingMelee false)))
      (Actor|DestroyActor _heldgun)
      (Variables|Default|SetWeaponSelected ""))))

(fn SwitchWeapon
  (params (WhichWeapon :type Integer))
  (if (Math|Boolean|ANDBoolean (!= WhichWeapon (Variables|Default|GetCurrWeapon)) (>= WhichWeapon 0) (< WhichWeapon (Utilities|Array|Length (Variables|Default|GetWeapons))))
    (Variables|Default|SetCurrWeapon WhichWeapon)
    (Weapon|DeselectWeapon)
    (bind _gunref (Weapon|EquipWeaponfromInventory WhichWeapon))
    (Variables|Default|SetHeldGun _gunref)))

(fn PrintWeapons
  (for (_array_element _array_index) (Variables|Default|GetWeapons)
    _))

(fn Interact
  (bind _firstpersoncamera (Variables|Default|GetFirstPersonCamera))
  ;[1 1 1] MLK: Really don't like looking for things this way, but for some reason other methods don't work for me...
  (bind (_outhits _returnvalue) (Collision|MultiSphereTraceForObjects (Transformation|GetWorldLocation (Variables|Default|GetFirstPersonCamera)) (+ (Transformation|GetWorldLocation _firstpersoncamera) (* (Math|Vector|GetForwardVector (Transformation|GetWorldRotation _firstpersoncamera)) (* (Components|Capsule|GetScaledCapsuleHalfHeight (Variables|Default|GetCapsuleComponent)) 2.0))) (Variables|Default|GetLookingRadius) (LocalVariables|GetLookForObjects) false (Utilities|Array|MakeArray (Variables|Default|GetHeldGun)) "Persistent"))
  (if _returnvalue
    (bind _array_element (Utilities|Array|ForEachLoopwithBreak _outhits :!label _label)
      (:LoopBody
        ;[1 1 1] Did we see a weapon? If some pick it up.
        (bind _asbp_weapon (Utilities|Casting|CastToBP_Weapon (.HitActor (Collision|BreakHitResult _array_element)))
          (:then
            (CallFunction|PickupWeapon _asbp_weapon)
            (goto _label Break))
          (:CastFailed
            ;[1 1 1] If not, did we see something interactable? If so interact with it.
            (if (Utilities|DoesObjectImplementInterface (.HitActor (Collision|BreakHitResult _array_element)) "/Game/_Blueprints/BPI_Stats.BPI_Stats_C")
              (Class|BPIStats|ButtonPressed(Message) (.HitActor (Collision|BreakHitResult _array_element)))
              (goto _label Break))))))))

(fn PrintWeaponInfo
  (params (Info :type Weapon%20Definition%20Structure))
  (Development|PrintString (Utilities|String|Append "ID: " (Utilities|String|ToString(Integer) (.id Info)) "Name: " (.name Info) "Is Ranged: " (Utilities|String|ToString(Boolean) (.isranged Info)) "Damage: " (Utilities|String|ToString(Integer) (.damage Info)))))

(fn DamagePlayer
  (params (Damage :type Integer))
  (Utilities|FlowControl|Sequence
    (:then_0
      (bind _output_get (Variables|Default|SetCurrHealth (- (Variables|Default|GetCurrHealth) Damage)))
      (CallFunction|OnHurt _output_get) ; This is to be overrided in ChildBP. This does sometihng cool when this gets hurt.
    )
    (:then_1
      (if (<= (Variables|Default|GetCurrHealth) 0)
        (CallFunction|OnKilled) ; This is to be overridded in childBP. This does something cool when thsi ies
      ))))

(fn PickupWeapon
  (params (Weapon :type BP%20Weapon%20Object%20Reference))
  (Weapon|PrintWeaponInfo (Variables|/Game/_Blueprints/Guns/BP_Weapon.BP_Weapon_C|GetWeaponInfo Weapon))
  (LocalVariables|SetWeaponInfo (Variables|/Game/_Blueprints/Guns/BP_Weapon.BP_Weapon_C|GetWeaponInfo Weapon))
  (Weapon|DeselectWeapon)
  (if (< (Variables|Default|GetWeaponsOwned) (Variables|Default|GetMaxWeapons))
    (Math|Integer|IncrementInt (Variables|Default|GetWeaponsOwned)
      (:%20%20
        (bind _result (Math|Integer|IncrementInt (Variables|Default|GetCurrWeapon))
          (:%20%20
            (Weapon|SetWeapon (LocalVariables|GetWeaponInfo) _result)))))
    (else
      (Weapon|SetWeapon (LocalVariables|GetWeaponInfo) (Variables|Default|GetCurrWeapon))))
  (bind _gunref (Weapon|SpawnWeapon (LocalVariables|GetWeaponInfo)))
  (Variables|Default|SetHeldGun _gunref))

(fn PrintCurrWeapon
  (Development|PrintString (Utilities|String|Append "Curr Weapon: " (Utilities|String|ToString(Integer) (Variables|Default|GetCurrWeapon)))))