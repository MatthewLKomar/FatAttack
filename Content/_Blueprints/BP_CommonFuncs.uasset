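; BP_CommonFuncs is a set of shared helper functions for loading screens, checkpoint loading and weapon data lookup.
; LoadFromCheckpoint adds the UI_Load widget to the viewport, then has BP_GameInstance load player data; its open-level-by-name nodes are left disconnected.
; LookUpFromData linearly scans Weapon_Table rows and returns the first whose ID field matches the given Id.
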(fn ShowLoadingScreen
  (bind _returnvalue (UserInterface|CreateWidget "/Game/UI/UI_Load.UI_Load_C"))
  (UserInterface|Viewport|AddtoViewport _returnvalue 0))

(fn LoadfromCheckpoint
  (CallFunction|ShowLoadingScreen)
  (bind _asbp_game_instance (Utilities|Casting|CastToBP_GameInstance (Game|GetGameInstance)))
  (Default|LoadPlayerData _asbp_game_instance))

(fn LookUpfromData
  (params (id :type Integer))
  (bind _outrownames (DataTable|GetDataTableRowNames "/Game/_Blueprints/Guns/Weapon_Table.Weapon_Table"))
  (bind _array_element (Utilities|Array|ForEachLoopwithBreak _outrownames :!label _label)
    (:LoopBody
      (bind _returnvalue (Utilities|GetDataTableRow "/Game/_Blueprints/Guns/Weapon_Table.Weapon_Table" _array_element)
        (:then
          (if (== (.ID (Utilities|Struct|BreakWeaponDefinition _returnvalue)) id)
            (LocalVariables|SetRetWeapon _returnvalue)
            (goto _label Break)))))
    (:Completed
      (return (LocalVariables|GetRetWeapon)))))