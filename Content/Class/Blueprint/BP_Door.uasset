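; Door actor that the player swings open or closed while standing inside its trigger box.
; Box overlap sets range flags, shows or removes the UI_Door prompt widget, and on entry starts a loop polling BP_Player's Open flag with short delays.
; A FlipFlop alternates timelines that yaw the door mesh forward or back.
; Timeline updates clear the player flag and re-enter the loop until the player leaves.
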(event OnComponentBeginOverlap(Box)
  (params (OverlappedComponent :type Primitive%20Component%20Object%20Reference) (OtherActor :type Actor%20Object%20Reference) (OtherComp :type Primitive%20Component%20Object%20Reference) (OtherBodyIndex :type Integer) (bFromSweep :type Boolean) (SweepResult :type Hit%20Result%20Structure%20%28by%20ref%29))
  (Variables|Default|SetCanOpen? true)
  (bind _returnvalue (UserInterface|CreateWidget "/Game/Class/Blueprint/UI_Door.UI_Door_C"))
  (UserInterface|Viewport|AddtoViewport _returnvalue 0)
  (CallFunction|Open?)
  (Variables|Default|SetLeave? false))

(event OnComponentEndOverlap(Box)
  (params (OverlappedComponent :type Primitive%20Component%20Object%20Reference) (OtherActor :type Actor%20Object%20Reference) (OtherComp :type Primitive%20Component%20Object%20Reference) (OtherBodyIndex :type Integer))
  (Variables|Default|SetCanOpen? false)
  (Widget|RemovefromParent (stale OnComponentBeginOverlap(Box) _returnvalue))
  (Variables|Default|SetLeave? true))

(event Custom|Open?
  (bind _sm_doorb (Variables|Default|GetSM_Doorb))
  (bind _asbp_player (Utilities|Casting|CastToBP_Player (Game|GetPlayerCharacter 0)))
  (Variables|/Game/Class/Blueprint/BP_Player.BP_Player_C|SetOpen _asbp_player false)
  (if (Variables|/Game/Class/Blueprint/BP_Player.BP_Player_C|GetOpen _asbp_player) :!label _label
    (if (Variables|Default|GetCanOpen?)
      (Utilities|FlowControl|FlipFlop
        (:A
          ;[1 1 1] Rot
          (bind _open (Timeline|Open PlayFromStart)
            (:Update
              (Transformation|SetRelativeRotation _sm_doorb (Math|Rotator|MakeRotator 0.0 0.0 _open) false false)
              (Variables|/Game/Class/Blueprint/BP_Player.BP_Player_C|SetOpen _asbp_player false))))
        (:B
          (bind _open_2 (Timeline|Timeline_0 ReverseFromEnd)
            (:Update
              (Transformation|SetRelativeRotation _sm_doorb (Math|Rotator|MakeRotator 0.0 0.0 _open_2) false false)
              (Variables|/Game/Class/Blueprint/BP_Player.BP_Player_C|SetOpen _asbp_player false)))))
      (if (not (Variables|Default|GetLeave?))
        (goto _label)))
    (else
      (Utilities|FlowControl|Delay 0.1)
      (if (not (Variables|Default|GetLeave?))
        (goto _label)))))

(event EventBeginPlay)

(event Collision|EventActorBeginOverlap
  (params (OtherActor :type Actor%20Object%20Reference)))

(fn ConstructionScript)