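; BP_Gun is a data-driven gun Blueprint that takes its definition and model from a weapon data table.
; Its construction script scans the table's rows for the first whose ID matches its own and stores that row as WeapInfo.
; It then applies the gun definition's model to the skeletal mesh.
; SetupWeapon and SetUpMuzzleForProjectile are empty stubs.
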(fn ConstructionScript
  (bind _outrownames (DataTable|GetDataTableRowNames "/Game/_Blueprints/Guns/Weapon_Table.Weapon_Table"))
  (bind _array_element (Utilities|Array|ForEachLoopwithBreak _outrownames :!label _label)
    (:LoopBody
      (bind _returnvalue (Utilities|GetDataTableRow "/Game/_Blueprints/Guns/Weapon_Table.Weapon_Table" _array_element)
        (:then
          (if (== (.ID (Utilities|Struct|BreakWeaponDefinition _returnvalue)) (Variables|Default|GetID))
            (Variables|Default|SetWeapInfo _returnvalue)
            (goto _label Break)))))
    (:Completed
      (Class|SkinnedMeshComponent|SetSkeletalMesh (Variables|Default|GetSkeletalMesh) (.Model (Utilities|Struct|BreakGunDefinitions (.GunDefinition (Utilities|Struct|BreakWeaponDefinition (Variables|Default|GetWeapInfo))))) true))))

(fn SetupWeapon
  (params (Info :type Weapon%20Definition%20Structure)))

(fn SetUpMuzzleforProjectile)