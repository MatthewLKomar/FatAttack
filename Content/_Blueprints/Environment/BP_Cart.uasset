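; BP_Cart is an environment cart that travels along the spline of a referenced track actor when active at BeginPlay.
; A timeline, with play rate set from Duration and starting time from an offset, outputs an alpha that maps to distance along the spline.
; Each update sets the cart's location and rotation to the world-space spline transform at that distance.
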(event Custom|MoveCart
  (Components|Timeline|SetPlayRate (Variables|Default|GetCartMover) (/ 1.0 (Variables|Default|GetDuration)))
  (Components|Timeline|SetNewTime (Variables|Default|GetCartMover) (Variables|Default|GetCartStartOffset))
  (bind _alpha (Timeline|CartMover Play)
    (:Update
      (Variables|Default|SetAlpha _alpha)
      (Transformation|SetActorLocationAndRotation (Spline|GetLocationatDistanceAlongSpline (Variables|/Game/_Blueprints/Environment/BP_Track.BP_Track_C|GetUseful%20Spline (Variables|Default|GetTrackRef)) (Math|Float|Lerp 0.0 (Spline|GetSplineLength (Variables|/Game/_Blueprints/Environment/BP_Track.BP_Track_C|GetUseful%20Spline (Variables|Default|GetTrackRef))) (Variables|Default|GetAlpha)) "World") (Spline|GetRotationatDistanceAlongSpline (Variables|/Game/_Blueprints/Environment/BP_Track.BP_Track_C|GetUseful%20Spline (Variables|Default|GetTrackRef)) (Math|Float|Lerp 0.0 (Spline|GetSplineLength (Variables|/Game/_Blueprints/Environment/BP_Track.BP_Track_C|GetUseful%20Spline (Variables|Default|GetTrackRef))) (Variables|Default|GetAlpha)) "World")))))

(event EventBeginPlay
  (if (Variables|Default|GetActiveCart)
    (CallFunction|MoveCart)))

(fn ConstructionScript)