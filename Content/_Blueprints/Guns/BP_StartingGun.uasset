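; BP_StartingGun is a gun that fires either a projectile or a hitscan shot, set by ProjectileBased.
; Shoot triggers the shot and GunEffects, holding IsShooting for GunAnimTime.
; Projectiles spawn offset along camera rotation; hitscan always takes the shotgun sphere trace, drawn persistently, damaging BPI_Stats actors.
; The unused line-trace branch has no endpoints wired and casts to BP_Creature, with a TODO to use an interface.
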(event EventBeginPlay)

(event Collision|EventActorBeginOverlap
  (params (OtherActor :type Actor%20Object%20Reference)))

(event EventTick
  (params (DeltaSeconds :type Float%20%28single-precision%29)))

(event EventShoot
  (Variables|Default|SetIsShooting true)
  (if (Variables|Default|GetProjectileBased)
    (CallFunction|GunFireProjectile "/Game/_Blueprints/Guns/BP_Projectile.BP_Projectile_C")
    (else
      (CallFunction|GunFireHitscan true)))
  (CallFunction|GunEffects)
  (Utilities|FlowControl|Delay (Variables|Default|GetGunAnimTime))
  (Variables|Default|SetIsShooting false))

(fn ConstructionScript
  (|CallParentFunction))

(fn GunFireProjectile
  (params (ProjectileClass :type Actor%20Class%20Reference))
  (bind _cameraref (Variables|Default|GetCameraRef))
  (bind _returnvalue (Transformation|GetWorldRotation _cameraref))
  (Game|SpawnActorfromClass ProjectileClass (Math|Transform|MakeTransform (+ (Transformation|GetWorldLocation (Variables|Default|GetSphere)) (Math|Vector|RotateVector (Variables|Default|GetGunOffset) _returnvalue)) _returnvalue) "AdjustIfPossibleButDontSpawnIfColliding" 0 0) ; Spawn projectile
)

(fn GunFireHitscan
  (params (Shotgun%20 :type Boolean))
  ;[1 1 1] TODO: CHANGE non shotgun to be an interface call instead of cast
  (if Shotgun%20
    ;[1 1 1] Sphere Trace. Will look like an "O"  and will pickup anything inside the "O"
    (bind (_outhit _returnvalue) (Collision|SphereTraceByChannel (Transformation|GetWorldLocation (Variables|Default|GetSphere)) (+ (Transformation|GetActorLocation) (* (Math|Vector|GetForwardVector (Variables|Default|GetCameraRef)) (Variables|Default|GetGunRange))) (Variables|Default|GetShotgunRadius) "TraceTypeQuery1" false 0 "Persistent"))
    (if _returnvalue ; We want to do an IF statement here just in case we don't hit anything so we don't risk breaking a null/nullptr value.
      (if (Utilities|DoesObjectImplementInterface (.HitActor (Collision|BreakHitResult _outhit)) "/Game/_Blueprints/BPI_Stats.BPI_Stats_C")
        ;[1 1 1] We checked to see if it contains the interface because we want to call an interface event on whoever we just shot.
        ;;[1 1 1] might not work
        (Class|BPIStats|Damage(Message) (.HitActor (Collision|BreakHitResult _outhit)) (Variables|Default|GetDamage))))
    (else
      (bind (_outhit_2 _returnvalue_2) (Collision|LineTraceByChannel "0, 0, 0" "0, 0, 0" "TraceTypeQuery1" false 0 "None"))
      (if _returnvalue_2
        ;[1 1 1] This will only work on BP_Creature and it's children. If we want to hurt a wall or another player this won't work. However if we called an interface function (like above) it would
        (bind _asbp_creature (Utilities|Casting|CastToBP_Creature (.HitActor (Collision|BreakHitResult _outhit_2))))
        (Default|DamageCreature _asbp_creature (Variables|Default|GetDamage))))))