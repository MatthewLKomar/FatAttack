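; BP_Creature is an enemy creature Blueprint, apparently a base, that provides stats and damage handling.
; On BeginPlay, SetStats picks the BP_EnemyStats row whose index matches CreatureType and copies its tactic, health and damage.
; Damage events call the empty OnHurt hook, then subtract from Health.
; The empty OnKilled hook fires when remaining Health is zero or above, so the death check appears inverted.
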(event EventBeginPlay
  (CallFunction|SetStats))

(event EventDamage
  (params (Damage :type Integer))
  (CallFunction|DamageCreature Damage))

(fn ConstructionScript)

(fn SetStats
  (bind _outrownames (DataTable|GetDataTableRowNames "/Game/_Blueprints/Enemies/EnemyStats/BP_EnemyStats.BP_EnemyStats"))
  (bind (_array_element _array_index) (Utilities|Array|ForEachLoopwithBreak _outrownames :!label _label)
    (:LoopBody
      (if (== _array_index (Math|Conversions|ToInteger(Byte) (Variables|EnemyDefinition|GetCreatureType)))
        (bind _returnvalue (Utilities|GetDataTableRow "/Game/_Blueprints/Enemies/EnemyStats/BP_EnemyStats.BP_EnemyStats" _array_element)
          (:then
            (Variables|EnemyDefinition|SetEnemyTactic (.tactic _returnvalue))
            (Variables|EnemyDefinition|SetHealth (.health _returnvalue))
            (Variables|EnemyDefinition|SetDamageGives (.damage _returnvalue))
            (goto _label Break)))))))

(fn DamageCreature
  (params (Damage :type Integer))
  (Utilities|FlowControl|Sequence
    (:then_0
      (CallFunction|OnHurt Damage) ; Does something cool when we get hurt
    )
    (:then_1
      (bind _output_get (Variables|EnemyDefinition|SetHealth (- (Variables|EnemyDefinition|GetHealth) Damage)))
      (if (>= _output_get 0)
        (CallFunction|OnKilled) ; Handles Death logic
      ))))

(fn OnHurt
  (params (DamageAmount :type Integer)))

(fn OnKilled)