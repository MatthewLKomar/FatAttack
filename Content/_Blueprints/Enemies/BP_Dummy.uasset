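; BP_Dummy is an enemy Blueprint that acts as a simple damageable dummy, with debug printing of its health and incoming damage.
; It extends a parent class, calling the parent's logic first in BeginPlay, OnHurt and OnKilled.
; It prints Health at BeginPlay and the damage amount in OnHurt, then destroys itself in OnKilled.
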(event EventBeginPlay
  (|CallParentFunction)
  (Development|PrintString (Utilities|String|ToString(Integer) (Variables|Default|GetHealth))))

(fn ConstructionScript
  (|CallParentFunction))

(fn OnHurt
  (params (DamageAmount :type Integer))
  (|CallParentFunction DamageAmount)
  (Development|PrintString (Utilities|String|ToString(Integer) DamageAmount)))

(fn OnKilled
  (|CallParentFunction)
  (Actor|DestroyActor))