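; Blackboard Blueprint that slides its right and left boards and switches the main board between screen and plain blackboard materials when key 2 is pressed.
; A FlipFlop alternates between two timeline pairs, with each right-board timeline's Update starting the left-board timeline that plays in the opposite direction.
; The left-board updates trigger a delayed material swap, then reset the DoOnce that blocks repeated presses.
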(event Input|KeyboardEvents|2
  (params (Key :type Key%20Structure))
  (bind _sm_blackbroad_main (Variables|Default|GetSM_Blackbroad_Main))
  (:Pressed
    (Utilities|FlowControl|DoOnce false :!label _label
      (:Completed
        (Utilities|FlowControl|FlipFlop
          (:A
            (bind _newtrack_0 (Timeline|Timeline_0 PlayFromStart)
              (:Update
                (Transformation|SetRelativeLocation (Variables|Default|GetSM_Blackbroad_R) _newtrack_0 false false)
                (bind _newtrack_0_2 (Timeline|Timeline_1 ReverseFromEnd)
                  (:Update
                    (Transformation|SetRelativeLocation (Variables|Default|GetSM_Blackbroad_L) _newtrack_0_2 false false)
                    (Utilities|FlowControl|Delay 3.0)
                    (Rendering|Material|SetMaterial _sm_blackbroad_main 1 "/Game/Class/Meterial/M_Blackboard_screen.M_Blackboard_screen")
                    (goto _label Reset))))))
          (:B
            (bind _newtrack_0_3 (Timeline|Timeline_3 ReverseFromEnd)
              (:Update
                (Transformation|SetRelativeLocation (Variables|Default|GetSM_Blackbroad_R) _newtrack_0_3 false false)
                (bind _newtrack_0_4 (Timeline|Timeline_2 PlayFromStart)
                  (:Update
                    (Transformation|SetRelativeLocation (Variables|Default|GetSM_Blackbroad_L) _newtrack_0_4 false false)
                    (Utilities|FlowControl|Delay 3.0)
                    (Rendering|Material|SetMaterial _sm_blackbroad_main 1 "/Game/Class/Meterial/M_Blackboard.M_Blackboard")
                    (goto _label Reset)))))))))))

(fn ConstructionScript)