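; Sinnamon roll enemy that extends a parent enemy class and performs its melee attack through an attached BP_Weapon.
; BeginPlay spawns the weapon and snaps it to the mesh, and MeleeAttack calls its Shoot after the parent logic.
; On death it spawns a weapon with a different ID at its location and destroys its own.
; Hurt and alert overrides add sounds; an unused Setup weapon spawn is noted as breaking AI Perception.
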(event EventBeginPlay
  (|CallParentFunction)
  (bind _returnvalue (Game|SpawnActorfromClass "/Game/_Blueprints/Guns/BP_Weapon.BP_Weapon_C" (Math|Transform|MakeTransform "0, 0, 0") "AlwaysSpawn" self (Variables|Default|GetScene) 9 false 0))
  (bind _output_get (Variables|Default|SetWeapon _returnvalue))
  (Transformation|AttachComponentToComponent _output_get (Variables|Character|GetMesh) "" "SnapToTarget" "SnapToTarget" "SnapToTarget" true))

(fn ConstructionScript
  (|CallParentFunction))

(fn Setup
  (|CallParentFunction))

(fn OnKilled
  (bind _weapon (Variables|Default|GetWeapon))
  (Game|SpawnActorfromClass "/Game/_Blueprints/Guns/BP_Weapon.BP_Weapon_C" (Math|Transform|MakeTransform (Transformation|GetActorLocation)) "AlwaysSpawn" 0 0 1 false 0)
  (Utilities|IsValid _weapon
    (:Is%20Valid
      (Actor|DestroyActor _weapon))
    (:Is%20Not%20Valid
      _))
  (|CallParentFunction))

(fn OnHurt
  (params (DamageAmount :type Integer))
  (|CallParentFunction DamageAmount)
  (Audio|PlaySoundatLocation "/Game/_Assets/SFX/SinammonRoll/SInnamonRoll_dMG.SInnamonRoll_dMG" (Transformation|GetActorLocation) "0, 0, 0" 1.0 1.0 0.0 "/Game/_Assets/SFX/SA_Master.SA_Master" 0 0))

(fn MeleeAttack
  (|CallParentFunction)
  (Default|Shoot (Variables|Default|GetWeapon)))

(fn PlayAlert
  (|CallParentFunction)
  (Audio|PlaySoundatLocation "/Game/_Assets/SFX/SinammonRoll/SC_SinnamonRoll_Alert.SC_SinnamonRoll_Alert" (Transformation|GetActorLocation) "0, 0, 0" 1.0 1.0 0.0 "/Game/_Assets/SFX/SA_Master.SA_Master" 0 0))