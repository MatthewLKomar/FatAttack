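; Macaroon enemy Blueprint that adds a spawned weapon and a ranged projectile attack to its parent enemy behavior.
; BeginPlay spawns a BP_Weapon attached to the mesh, which melee attacks fire via Shoot and OnKilled destroys.
; Ranged throws bypass the parent and weapon, calling ShootProjectile from the Scene component.
; OnHurt prints health for debugging, and a disconnected weapon spawn in Setup is noted as breaking AI Perception.
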(event EventBeginPlay
  (|CallParentFunction)
  (bind _returnvalue (Game|SpawnActorfromClass "/Game/_Blueprints/Guns/BP_Weapon.BP_Weapon_C" (Math|Transform|MakeTransform "0, 0, 0") "AlwaysSpawn" self (Variables|Default|GetScene) 9 false 0))
  (bind _output_get (Variables|Default|SetWeapon _returnvalue))
  (Transformation|AttachComponentToComponent _output_get (Variables|Character|GetMesh) "" "SnapToTarget" "SnapToTarget" "SnapToTarget" true))

(fn ConstructionScript
  (|CallParentFunction))

(fn Setup
  (|CallParentFunction))

(fn OnKilled
  (bind _weapon (Variables|Default|GetWeapon))
  (Utilities|IsValid _weapon
    (:Is%20Valid
      (Actor|DestroyActor _weapon))
    (:Is%20Not%20Valid
      _))
  (|CallParentFunction))

(fn ThrowRangedItem
  (CallFunction|ShootProjectile 4 (Variables|Default|GetScene)))

(fn OnHurt
  (params (DamageAmount :type Integer))
  (|CallParentFunction DamageAmount)
  (Development|PrintString (Utilities|String|Append "New Health" (Utilities|String|ToString(Integer) (Variables|Default|GetHealth)))))

(fn MeleeAttack
  (|CallParentFunction)
  (Default|Shoot (Variables|Default|GetWeapon)))