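; Data-driven weapon actor that looks up its stats in Weapon_Table by ID during construction, sets its mesh and snaps a muzzle sphere to ranged models.
; Shoot either spawns BP_GenericProjectile or runs a multi-sphere trace from the muzzle along the owner's head direction, using shotgun spread as radius.
; Trace hits, deduplicated through HurtActors, and mesh overlaps while equipped deal damage through the BPI_Stats DamageMessage interface.
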(event OnComponentBeginOverlap(SkeletalMesh)
  (params (OverlappedComponent :type Primitive%20Component%20Object%20Reference) (OtherActor :type Actor%20Object%20Reference) (OtherComp :type Primitive%20Component%20Object%20Reference) (OtherBodyIndex :type Integer) (bFromSweep :type Boolean) (SweepResult :type Hit%20Result%20Structure%20%28by%20ref%29))
  (if (and (Variables|Default|GetIsEquipped) (!= OtherActor (Game|GetInstigator)))
    ;[1 1 1] Add Damage
    (if (Utilities|DoesObjectImplementInterface OtherActor "/Game/_Blueprints/BPI_Stats.BPI_Stats_C")
      (Class|BPIStats|Damage(Message) OtherActor (.Damage (Utilities|Struct|BreakWeaponDefinition (Variables|Default|GetWeaponInfo)))))))

(event Custom|Shoot
  (bind _weaponinfo (Variables|Default|GetWeaponInfo))
  (bind (_id _name _damage _isranged _gundefinition) (Utilities|Struct|BreakWeaponDefinition _weaponinfo))
  ;[1 1 1] Do stuff here
  (if _isranged
    (if (.isProjectile (Utilities|Struct|BreakGunDefinitions _gundefinition))
      (CallFunction|GunFireProjectile)
      (else
        (CallFunction|GunFireHitscan true)))))

(event EventBeginPlay)

(fn ConstructionScript
  (bind _outrownames (DataTable|GetDataTableRowNames "/Game/_Blueprints/Guns/Weapon_Table.Weapon_Table"))
  (bind _array_element (Utilities|Array|ForEachLoopwithBreak _outrownames :!label _label)
    (:LoopBody
      (bind _returnvalue (Utilities|GetDataTableRow "/Game/_Blueprints/Guns/Weapon_Table.Weapon_Table" _array_element)
        (:then
          (if (== (.ID (Utilities|Struct|BreakWeaponDefinition _returnvalue)) (Variables|Default|GetID))
            (Variables|Default|SetWeaponInfo _returnvalue)
            (goto _label Break)))))
    (:Completed
      (CallFunction|SetupWeapon (Variables|Default|GetWeaponInfo))
      (CallFunction|SetUpMuzzleforProjectile))))

(fn GunEffects
  (Audio|PlaySoundatLocation "/Game/_Assets/DefaultFirstPerson/Audio/FirstPersonTemplateWeaponFire02.FirstPersonTemplateWeaponFire02" (Transformation|GetActorLocation) "0, 0, 0" 1.0 1.0 0.0 0 0 0) ; Play firing sound
)

(fn SetupWeapon
  (params (Info :type Weapon%20Definition%20Structure))
  (Class|SkinnedMeshComponent|SetSkeletalMesh (Variables|Default|GetSkeletalMesh) (.Model (Utilities|Struct|BreakGunDefinitions (.GunDefinition (Utilities|Struct|BreakWeaponDefinition Info)))) true)
  (if (not (.isRanged (Utilities|Struct|BreakWeaponDefinition Info)))
    (Collision|SetCollisionEnabled (Variables|Default|GetCapsule) "NoCollision")
    (Collision|SetCollisionEnabled (Variables|Default|GetSphere) "NoCollision")))

(fn GunFireProjectile
  (bind _weaponinfo (Variables|Default|GetWeaponInfo))
  (bind _projectileinfo (Utilities|Struct|BreakGunDefinitions (.gundefinition _weaponinfo)))
  (bind (_projectile _projectilespeed _projectileimpactdecal _isexplosive _isgrenade) (Utilities|Struct|BreakProjectileDefinitions _projectileinfo))
  (Game|SpawnActorfromClass "/Game/_Blueprints/Guns/BP_GenericProjectile.BP_GenericProjectile_C" (Math|Transform|MakeTransform (Transformation|GetWorldLocation (Variables|Default|GetSphere)) (Transformation|GetWorldRotation (Variables|Default|GetOwnerHeadTransform))) "AlwaysSpawn" 0 (Variables|Default|GetID) false 0 _isexplosive _isgrenade self 0) ; Spawn projectile
)

(fn GunFireHitscan
  (params (Shotgun%20 :type Boolean))
  (Utilities|Array|Add (LocalVariables|GetIgnoreActors) (Components|GetOwner (Variables|Default|GetOwnerHeadTransform)))
  (if Shotgun%20
    _
    (else
      _))
  ;[1 1 1] Sphere Trace. Will look like an "O"  and will pickup anything inside the "O"
  (bind (_outhits _returnvalue) (Collision|MultiSphereTraceByChannel (Transformation|GetWorldLocation (Variables|Default|GetSphere)) (+ (Transformation|GetWorldLocation (Variables|Default|GetSphere)) (* (Math|Vector|GetForwardVector (Variables|Default|GetOwnerHeadTransform)) (.Range (Utilities|Struct|BreakGunDefinitions (.GunDefinition (Utilities|Struct|BreakWeaponDefinition (Variables|Default|GetWeaponInfo))))))) (.ShotgunSpread (Utilities|Struct|BreakGunDefinitions (.GunDefinition (Utilities|Struct|BreakWeaponDefinition (Variables|Default|GetWeaponInfo))))) "TraceTypeQuery3" false (LocalVariables|GetIgnoreActors) "Persistent"))
  (if _returnvalue ; We want to do an IF statement here just in case we don't hit anything so we don't risk breaking a null/nullptr value.
    (for _array_element _outhits
      (if (Utilities|DoesObjectImplementInterface (.HitActor (Collision|BreakHitResult _array_element)) "/Game/_Blueprints/BPI_Stats.BPI_Stats_C")
        (Utilities|IsValid (.HitActor (Collision|BreakHitResult _array_element))
          (:Is%20Valid
            (Utilities|AddDamagedActors (LocalVariables|GetHurtActors) (.HitActor (Collision|BreakHitResult _array_element)))))))
    (for _array_element_2 (LocalVariables|GetHurtActors)
      (Utilities|IsValid _array_element_2
        (:Is%20Valid
          (Class|BPIStats|Damage(Message) _array_element_2 (.Damage (Utilities|Struct|BreakWeaponDefinition (Variables|Default|GetWeaponInfo)))))))))

(fn SetUpMuzzleforProjectile
  (bind _skeletalmesh (Variables|Default|GetSkeletalMesh))
  (if (Math|Boolean|ANDBoolean (.isRanged (Utilities|Struct|BreakWeaponDefinition (Variables|Default|GetWeaponInfo))) (Utilities|IsValid _skeletalmesh) (Transformation|DoesSocketExist _skeletalmesh "Muzzle"))
    (Transformation|AttachComponentToComponent (Variables|Default|GetSphere) (Variables|Default|GetSkeletalMesh) "Muzzle" "SnapToTarget" "SnapToTarget" "SnapToTarget" true)
    (Transformation|SetWorldScale3D (Variables|Default|GetSphere) "0.100000,0.100000,0.100000")))