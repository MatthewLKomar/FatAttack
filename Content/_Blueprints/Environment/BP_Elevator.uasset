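; Elevator Blueprint with sliding double doors that carries a platform upward when its trigger is overlapped.
; Entry and exit triggers open and close the doors with timelines that lerp relative locations, with a delay before exit opening.
; The platform trigger closes the entry doors, waits, then raises platform and both doors on parallel timelines.
; The graph has no logic to send the platform back down.
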(event OnComponentBeginOverlap(DoorEnter)
  (params (OverlappedComponent :type Primitive%20Component%20Object%20Reference) (OtherActor :type Actor%20Object%20Reference) (OtherComp :type Primitive%20Component%20Object%20Reference) (OtherBodyIndex :type Integer) (bFromSweep :type Boolean) (SweepResult :type Hit%20Result%20Structure%20%28by%20ref%29))
  ;[1 1 1] Someone is near, open door
  (Utilities|FlowControl|Sequence
    (:then_0
      (bind _newtrack_0 (Timeline|Left%20Door%20Enter Play)
        (:Update
          (Transformation|SetRelativeLocation (Variables|Default|GetLeft%20Door) (Math|Vector|Lerp(Vector) (Variables|Default|GetLeft%20Door%20Enter%20Start) (Variables|Default|GetLeft%20Door%20Enter%20End) _newtrack_0) false false))))
    (:then_1
      ;[1 1 1] Someone left the door
      (bind _newtrack_0_2 (Timeline|Right%20Door%20Enter Play)
        (:Update
          (Transformation|SetRelativeLocation (Variables|Default|GetRight%20Door) (Math|Vector|Lerp(Vector) (Variables|Default|GetRight%20Door%20Enter%20Start) (Variables|Default|GetRight%20Door%20Enter%20End) _newtrack_0_2) false false))))))

(event OnComponentEndOverlap(DoorEnter)
  (params (OverlappedComponent :type Primitive%20Component%20Object%20Reference) (OtherActor :type Actor%20Object%20Reference) (OtherComp :type Primitive%20Component%20Object%20Reference) (OtherBodyIndex :type Integer))
  ;[1 1 1] Someone left the door
  (Utilities|FlowControl|Sequence
    (:then_0
      ;[1 1 1] Someone is near, open door
      (bind _newtrack_0 (Timeline|Left%20Door%20Enter Reverse)
        (:Update
          (Transformation|SetRelativeLocation (Variables|Default|GetLeft%20Door) (Math|Vector|Lerp(Vector) (Variables|Default|GetLeft%20Door%20Enter%20Start) (Variables|Default|GetLeft%20Door%20Enter%20End) _newtrack_0) false false))))
    (:then_1
      (bind _newtrack_0_2 (Timeline|Right%20Door%20Enter Reverse)
        (:Update
          (Transformation|SetRelativeLocation (Variables|Default|GetRight%20Door) (Math|Vector|Lerp(Vector) (Variables|Default|GetRight%20Door%20Enter%20Start) (Variables|Default|GetRight%20Door%20Enter%20End) _newtrack_0_2) false false))))))

(event OnComponentBeginOverlap(PlatformTrigger)
  (params (OverlappedComponent :type Primitive%20Component%20Object%20Reference) (OtherActor :type Actor%20Object%20Reference) (OtherComp :type Primitive%20Component%20Object%20Reference) (OtherBodyIndex :type Integer) (bFromSweep :type Boolean) (SweepResult :type Hit%20Result%20Structure%20%28by%20ref%29))
  ;[1 1 1] Someone's on the elevatore so move up
  (Utilities|FlowControl|Sequence
    (:then_0
      ;[1 1 1] Someone left the door
      (Utilities|FlowControl|Sequence
        (:then_0
          ;[1 1 1] Someone is near, open door
          (bind _newtrack_0 (Timeline|Left%20Door%20Enter Reverse)
            (:Update
              (Transformation|SetRelativeLocation (Variables|Default|GetLeft%20Door) (Math|Vector|Lerp(Vector) (Variables|Default|GetLeft%20Door%20Enter%20Start) (Variables|Default|GetLeft%20Door%20Enter%20End) _newtrack_0) false false))))
        (:then_1
          (bind _newtrack_0_2 (Timeline|Right%20Door%20Enter Reverse)
            (:Update
              (Transformation|SetRelativeLocation (Variables|Default|GetRight%20Door) (Math|Vector|Lerp(Vector) (Variables|Default|GetRight%20Door%20Enter%20Start) (Variables|Default|GetRight%20Door%20Enter%20End) _newtrack_0_2) false false))))))
    (:then_1
      (Utilities|FlowControl|Delay 4.0)
      (Utilities|FlowControl|Sequence
        (:then_0
          (bind _newtrack_1 (Timeline|Platform%20Up Play)
            (:Update
              (Transformation|SetRelativeLocation (Variables|Default|GetPlatform) (Math|Vector|Lerp(Vector) (Variables|Default|GetPlatform%20Start) (Variables|Default|GetPlatform%20End) _newtrack_1) false false))))
        (:then_1
          (bind _newtrack_0_3 (Timeline|Left%20Up Play)
            (:Update
              (Transformation|SetRelativeLocation (Variables|Default|GetLeft%20Door) (Math|Vector|Lerp(Vector) (Variables|Default|GetLeft%20Door%20Enter%20Start) (Variables|Default|GetLeft%20Door%20Up) _newtrack_0_3) false false))))
        (:then_2
          (bind _newtrack_0_4 (Timeline|Right%20Up Play)
            (:Update
              (Transformation|SetRelativeLocation (Variables|Default|GetRight%20Door) (Math|Vector|Lerp(Vector) (Variables|Default|GetRight%20Door%20Enter%20Start) (Variables|Default|GetRight%20Door%20Up) _newtrack_0_4) false false))))))))

(event OnComponentBeginOverlap(DoorExit)
  (params (OverlappedComponent :type Primitive%20Component%20Object%20Reference) (OtherActor :type Actor%20Object%20Reference) (OtherComp :type Primitive%20Component%20Object%20Reference) (OtherBodyIndex :type Integer) (bFromSweep :type Boolean) (SweepResult :type Hit%20Result%20Structure%20%28by%20ref%29))
  ;[1 1 1] We've arrived so open the doors
  (Utilities|FlowControl|Delay 3.0)
  (Utilities|FlowControl|Sequence
    (:then_0
      (bind _newtrack_0 (Timeline|Left%20Door%20Exit Play)
        (:Update
          (Transformation|SetRelativeLocation (Variables|Default|GetLeft%20Door) (Math|Vector|Lerp(Vector) (Variables|Default|GetLeft%20Door%20Up) (Variables|Default|GetLeft%20Door%20Up%20End) _newtrack_0) false false))))
    (:then_1
      (bind _newtrack_0_2 (Timeline|Right%20Door%20Exit Play)
        (:Update
          (Transformation|SetRelativeLocation (Variables|Default|GetRight%20Door) (Math|Vector|Lerp(Vector) (Variables|Default|GetRight%20Door%20Up) (Variables|Default|GetRight%20Door%20Up%20End) _newtrack_0_2) false false))))))

(event OnComponentEndOverlap(DoorExit)
  (params (OverlappedComponent :type Primitive%20Component%20Object%20Reference) (OtherActor :type Actor%20Object%20Reference) (OtherComp :type Primitive%20Component%20Object%20Reference) (OtherBodyIndex :type Integer))
  ;[1 1 1] We've arrived so open the doors
  (Utilities|FlowControl|Sequence
    (:then_0
      (bind _newtrack_0 (Timeline|Left%20Door%20Exit Reverse)
        (:Update
          (Transformation|SetRelativeLocation (Variables|Default|GetLeft%20Door) (Math|Vector|Lerp(Vector) (Variables|Default|GetLeft%20Door%20Up) (Variables|Default|GetLeft%20Door%20Up%20End) _newtrack_0) false false))))
    (:then_1
      (bind _newtrack_0_2 (Timeline|Right%20Door%20Exit Reverse)
        (:Update
          (Transformation|SetRelativeLocation (Variables|Default|GetRight%20Door) (Math|Vector|Lerp(Vector) (Variables|Default|GetRight%20Door%20Up) (Variables|Default|GetRight%20Door%20Up%20End) _newtrack_0_2) false false))))))

(fn ConstructionScript)