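; Game instance that manages save games, loading or creating a BP_FFSaveObj on Init and keeping it as SaveGameData.
; SavePlayerData writes the player's health, transform and level name to the slot, while ClearSaveData deletes it.
; LoadPlayerData restores transform and health, then on a level mismatch opens a level named by SaveSlotName, not the saved level.
; Level-data functions are empty stubs, and the looping AutoSave timer is unconnected.
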(event Custom|LoadGame
  (params (SaveSlotName :type String))
  ;[1 1 1] If you want to have a Load a save menu
  ; use this
  (bind _returnvalue (SaveGame|DoesSaveGameExist SaveSlotName)) ; slot name is the name of the file name
  (if _returnvalue
    (bind _returnvalue_2 (SaveGame|LoadGamefromSlot (Variables|Default|GetSaveSlotName)))
    (bind _asbp_ffsave_obj (Utilities|Casting|CastToBP_FFSaveObj _returnvalue_2))
    (Variables|Default|SetSaveGameData _asbp_ffsave_obj)
    (else
      ;[1 1 1] If there isn't a save file, create a new one
      (bind _returnvalue_3 (SaveGame|CreateSaveGameObject "/Game/_Blueprints/SaveLogic/BP_FFSaveObj.BP_FFSaveObj_C"))
      (Variables|Default|SetSaveGameData _returnvalue_3))))

(event EventInit
  (SaveGame|DoesSaveGameExist (Variables|Default|GetSaveSlotName)) ; slot name is the name of the file name
  (if (stale Custom|LoadGame _returnvalue)
    (bind _returnvalue (SaveGame|LoadGamefromSlot (Variables|Default|GetSaveSlotName)))
    (bind _asbp_ffsave_obj (Utilities|Casting|CastToBP_FFSaveObj _returnvalue))
    (Variables|Default|SetSaveGameData _asbp_ffsave_obj)
    (else
      ;[1 1 1] If there isn't a save file, create a new one
      (bind _returnvalue_2 (SaveGame|CreateSaveGameObject "/Game/_Blueprints/SaveLogic/BP_FFSaveObj.BP_FFSaveObj_C"))
      (Variables|Default|SetSaveGameData _returnvalue_2))))

(fn SavePlayerData
  (bind _asbp_player (Utilities|Casting|CastToBP_Player (Game|GetPlayerCharacter 0)))
  (bind _returnvalue (Game|GetCurrentLevelName true))
  (bind _output_get (LocalVariables|SetPlayer _asbp_player))
  (Variables|/Game/_Blueprints/SaveLogic/BP_FFSaveObj.BP_FFSaveObj_C|SetPlayerData (Variables|Default|GetSaveGameData) (Utilities|Struct|MakeFPlayerSaveData (Variables|/Game/_Blueprints/Player/BP_Player.BP_Player_C|GetCurrHealth _output_get) (Transformation|GetActorTransform _asbp_player) 0 _returnvalue 0 0.0 0))
  (SaveGame|SaveGametoSlot (Variables|Default|GetSaveGameData) (Variables|Default|GetSaveSlotName)))

(fn LoadPlayerData
  (bind _asbp_player (Utilities|Casting|CastToBP_Player (Game|GetPlayerCharacter 0)))
  (LocalVariables|SetPlayer _asbp_player)
  (bind _savegamedata (Variables|Default|GetSaveGameData)
    (:then
      (Utilities|FlowControl|Sequence
        (:then_0
          (Transformation|SetActorTransform (LocalVariables|GetPlayer) (.playertransform (Variables|/Game/_Blueprints/SaveLogic/BP_FFSaveObj.BP_FFSaveObj_C|GetPlayerData _savegamedata))))
        (:then_1
          (Variables|/Game/_Blueprints/Player/BP_Player.BP_Player_C|SetCurrHealth (LocalVariables|GetPlayer) (.playerhealth (Variables|/Game/_Blueprints/SaveLogic/BP_FFSaveObj.BP_FFSaveObj_C|GetPlayerData _savegamedata))))
        (:then_2
          (bind _returnvalue (Game|GetCurrentLevelName true))
          (if (not (Utilities|Enum|Equal(Enum) (.playerlevel (Variables|/Game/_Blueprints/SaveLogic/BP_FFSaveObj.BP_FFSaveObj_C|GetPlayerData _savegamedata)) _returnvalue))
            (Game|OpenLevel(byName) (Utilities|String|StringToName (Variables|Default|GetSaveSlotName)))))))
    (:else)))

(fn LoadLevelData)

(fn SaveLevelData)

(fn AutoSave
  (CallFunction|SavePlayerData))

(fn ClearSaveData
  (SaveGame|DeleteGameinSlot (Variables|Default|GetSaveSlotName)))