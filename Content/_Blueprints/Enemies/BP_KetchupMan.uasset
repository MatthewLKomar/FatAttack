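; BP_KetchupMan is an enemy Blueprint that explodes when killed, damaging nearby actors.
; OnKilled sphere-traces at the mesh within BlastRadius and uses AddPeopleSeen to collect each BPI_Stats actor once into HurtActors.
; Each collected actor receives a flat 40 damage via DamageMessage before the parent death logic runs.
; A debug sphere still draws on death, and the CalculateBlastDamage formula is left unconnected as a TODO.
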(event EventBeginPlay
  (|CallParentFunction))

(event Collision|EventActorBeginOverlap
  (params (OtherActor :type Actor%20Object%20Reference)))

(event EventTick
  (params (DeltaSeconds :type Float%20%28single-precision%29)))

(fn ConstructionScript
  (|CallParentFunction))

(fn OnKilled
  (bind _mesh (Variables|Character|GetMesh))
  (bind _returnvalue (Transformation|GetWorldLocation _mesh))
  (Rendering|Debug|DrawDebugSphere (Transformation|GetWorldLocation (Variables|Character|GetMesh)) 2e+01 12 "(R=1.000000,G=0.000000,B=0.394385,A=1.000000)" 2e+01 2e+01)
  (bind (_outhits _returnvalue_2) (Collision|MultiSphereTraceForObjects _returnvalue _returnvalue (Variables|Default|GetBlastRadius) (Variables|Default|GetObject%20Types) false 0 "None"))
  (if _returnvalue_2
    (for _array_element _outhits
      (if (Utilities|DoesObjectImplementInterface (.HitActor (Collision|BreakHitResult _array_element)) "/Game/_Blueprints/BPI_Stats.BPI_Stats_C")
        (Utilities|IsValid (.HitActor (Collision|BreakHitResult _array_element))
          (:Is%20Valid
            (Utilities|AddPeopleSeen (LocalVariables|GetHurtActors) (.HitActor (Collision|BreakHitResult _array_element)))))))
    (for _array_element_2 (LocalVariables|GetHurtActors)
      (Utilities|IsValid _array_element_2
        (:Is%20Valid
          (Class|BPIStats|Damage(Message) _array_element_2 40))))
    (|CallParentFunction)
    (else
      (|CallParentFunction))))

(fn OnHurt
  (params (DamageAmount :type Integer))
  (|CallParentFunction DamageAmount))