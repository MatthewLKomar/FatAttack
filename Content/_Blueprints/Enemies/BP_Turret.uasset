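; BP_Turret is an enemy turret Blueprint that fires through a separately spawned weapon actor.
; On BeginPlay it spawns a BP_Weapon at the mesh's GripPoint socket, passing its Scene component as the owner head transform, and stores the reference.
; RangedAttack calls the parent logic, then tells that weapon to shoot; OnKilled only defers to the parent.
; A direct ShootProjectile call remains in RangedAttack but is disconnected.
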(event EventBeginPlay
  (|CallParentFunction)
  (bind _returnvalue (Game|SpawnActorfromClass "/Game/_Blueprints/Guns/BP_Weapon.BP_Weapon_C" (Math|Transform|MakeTransform (Transformation|GetSocketLocation (Variables|Character|GetMesh) "GripPoint") (Transformation|GetWorldRotation (Variables|Default|GetScene))) "AlwaysSpawn" 0 (Variables|Default|GetScene) 6 false 0))
  (Variables|Default|SetWeapon _returnvalue))

(fn ConstructionScript
  (|CallParentFunction))

(fn OnKilled
  (|CallParentFunction))

(fn RangedAttack
  (|CallParentFunction)
  (Default|Shoot (Variables|Default|GetWeapon)))