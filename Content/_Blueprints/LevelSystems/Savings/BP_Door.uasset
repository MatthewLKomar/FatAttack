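; BP_Door is a door in the level saving system that opens once when the player overlaps its box.
; The overlap calls OpenDoor, which plays a timeline to move the Cube, then sets IsOpen and reports the door to MyGameState through CallDoorOpened.
; BeginPlay and UpdateDoor snap the Cube to its lowered position when IsOpen is already true, restoring the open state without animation.
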(event OnComponentBeginOverlap(Box)
  (params (OverlappedComponent :type Primitive%20Component%20Object%20Reference) (OtherActor :type Actor%20Object%20Reference) (OtherComp :type Primitive%20Component%20Object%20Reference) (OtherBodyIndex :type Integer) (bFromSweep :type Boolean) (SweepResult :type Hit%20Result%20Structure%20%28by%20ref%29))
  (Utilities|Casting|CastToBP_Player OtherActor)
  (CallFunction|OpenDoor))

(event Custom|OpenDoor
  (if (not (Variables|Default|GetIsOpen))
    (bind _vector (Timeline|Timeline_0 Play)
      (:Update
        (Transformation|SetRelativeLocation (Variables|Default|GetCube) _vector false false))
      (:Finished
        (Variables|Default|SetIsOpen true)
        (bind _asmy_game_state (Utilities|Casting|CastToMyGameState (Game|GetGameState)))
        (Default|CallDoorOpened _asmy_game_state self)))))

(event Custom|UpdateDoor
  (if (Variables|Default|GetIsOpen)
    (Transformation|SetRelativeLocation (Variables|Default|GetCube) "0, 0,-300.000000" false false)))

(event Collision|EventActorBeginOverlap
  (params (OtherActor :type Actor%20Object%20Reference)))

(event EventTick
  (params (DeltaSeconds :type Float%20%28single-precision%29)))

(event EventBeginPlay
  (if (Variables|Default|GetIsOpen)
    (Transformation|SetRelativeLocation (Variables|Default|GetCube) "0, 0,-300.000000" false false)))

(fn ConstructionScript)