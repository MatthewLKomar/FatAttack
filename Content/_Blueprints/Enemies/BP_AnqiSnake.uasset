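; BP_AnqiSnake is a child enemy Blueprint with melee and ranged attacks, voiced by pizza-named sounds.
; It overrides parent hooks for idle, melee, hurt, death and throwing to add sounds; throwing fires a projectile directly without calling the parent.
; A Box overlap damages BPI_Stats actors during melee, independent of animation timing.
; Weapon spawning in Setup is disconnected, noted as breaking AI Perception.
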(event OnComponentBeginOverlap(Box)
  (params (OverlappedComponent :type Primitive%20Component%20Object%20Reference) (OtherActor :type Actor%20Object%20Reference) (OtherComp :type Primitive%20Component%20Object%20Reference) (OtherBodyIndex :type Integer) (bFromSweep :type Boolean) (SweepResult :type Hit%20Result%20Structure%20%28by%20ref%29))
  ;[1 1 1] This just hurts the enemy if we're melee attacking and if they're next to us, but this isn't dependent on the stage in the animation
  (if (Math|Boolean|ANDBoolean (!= OtherActor self) (Variables|Default|GetIsMeleeAttack) (Utilities|DoesObjectImplementInterface OtherActor "/Game/_Blueprints/BPI_Stats.BPI_Stats_C"))
    (Class|BPIStats|Damage(Message) OtherActor (Variables|Default|GetDamageGives))))

(event EventBeginPlay
  (|CallParentFunction))

(event Collision|EventActorBeginOverlap
  (params (OtherActor :type Actor%20Object%20Reference)))

(event EventTick
  (params (DeltaSeconds :type Float%20%28single-precision%29)))

(fn ConstructionScript
  (|CallParentFunction))

(fn Setup
  (|CallParentFunction))

(fn OnKilled
  (bind _weapon (Variables|Default|GetWeapon))
  (Utilities|IsValid _weapon
    (:Is%20Valid
      (Actor|DestroyActor _weapon))
    (:Is%20Not%20Valid
      _))
  (Audio|PlaySoundatLocation "/Game/_Assets/SFX/Pizza/SC_PizzaDie.SC_PizzaDie" (Transformation|GetActorLocation) "0, 0, 0" 1.0 1.0 0.0 "/Game/_Assets/SFX/SA_Master.SA_Master" 0 0)
  (|CallParentFunction))

(fn ThrowRangedItem
  (Audio|PlaySoundatLocation "/Game/_Assets/SFX/Pizza/SC_PizzaThrow.SC_PizzaThrow" (Transformation|GetActorLocation) "0, 0, 0" 1.0 1.0 0.0 "/Game/_Assets/SFX/SA_Master.SA_Master" 0 0)
  (CallFunction|ShootProjectile 4 (Variables|Default|GetScene)))

(fn OnHurt
  (params (DamageAmount :type Integer))
  (|CallParentFunction DamageAmount)
  (Audio|PlaySoundatLocation "/Game/_Assets/SFX/Pizza/SC_PizzaDmg.SC_PizzaDmg" (Transformation|GetActorLocation) "0, 0, 0" 1.0 1.0 0.0 "/Game/_Assets/SFX/SA_Master.SA_Master" 0 0))

(fn MeleeAttack
  (|CallParentFunction)
  (Audio|PlaySoundatLocation "/Game/_Assets/SFX/Pizza/SC_PizzaButt.SC_PizzaButt" (Transformation|GetActorLocation) "0, 0, 0" 1.0 1.0 0.0 0 0 0))

(fn PlayIdle
  (|CallParentFunction)
  (Audio|PlaySoundatLocation "/Game/_Assets/SFX/Pizza/pizza_face_idle.pizza_face_idle" (Transformation|GetActorLocation) "0, 0, 0" 1.0 1.0 0.0 "/Game/_Assets/SFX/SA_Master.SA_Master" 0 0))